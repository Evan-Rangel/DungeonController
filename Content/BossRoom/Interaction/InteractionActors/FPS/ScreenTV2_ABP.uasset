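; ScreenTV2_ABP is an interactable TV screen actor in the BossRoom area whose displayed material toggles when used.
; Interface events toggle custom-depth rendering on the Cube mesh for focus and forward interaction to InteractOnServer, which flips the InteractToggle boolean.
; The InteractToggle RepNotify then swaps the mesh material between StaticTV_M when true and BattleTV_M when false.
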(event Custom|InteractOnServer
  (Variables|Default|SetInteractToggle (not (Variables|Default|GetInteractToggle))))

(event EventBeginPlay)

(event Collision|EventActorBeginOverlap
  (params (OtherActor :type Actor%20Object%20Reference)))

(event EventTick
  (params (DeltaSeconds :type Float%20%28single-precision%29)))

(event EventInterfaceToggleFocus
  (params (Focus :type Boolean))
  (Rendering|SetRenderCustomDepth (Variables|Default|GetCube) Focus))

(event EventInterfaceInteract
  (CallFunction|InteractonServer))

(fn ConstructionScript)

(fn OnRepInteractToggle
  ;[0 0 0] Aqui es donde se debe poner la accion a realizar una vez se pulse el boton, si se pulsa es "True" si se vuelve a pulsar es "False".
  (if (Variables|Default|GetInteractToggle)
    (Rendering|Material|SetMaterial (Variables|Default|GetCube) 0 "/Game/BossRoom/SecurityCameras/Materials/StaticTV_M.StaticTV_M")
    (else
      (Rendering|Material|SetMaterial (Variables|Default|GetCube) 0 "/Game/BossRoom/SecurityCameras/Materials/BattleTV_M.BattleTV_M"))))
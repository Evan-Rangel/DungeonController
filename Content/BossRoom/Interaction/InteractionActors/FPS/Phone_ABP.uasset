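; Interactable boss room phone that rings from BeginPlay and opens a dialogue HUD when answered.
; Focus toggles a custom depth highlight on its mesh, and interacting calls InteractOnServer, which flips InteractToggle unless already InPhone.
; The OnRep handler stops the ringing, sets InPhone, fades room music unless GanasteMusic is set, then creates the dialogue widget and registers it with Battle_GM.
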(event Custom|InteractOnServer
  (if (not (Variables|Default|GetInPhone))
    (Variables|Default|SetInteractToggle (not (Variables|Default|GetInteractToggle)))))

(event EventBeginPlay
  (bind _cube (Variables|Default|GetCube))
  (bind _asboss_first_person_player_bp (Utilities|Casting|CastToBossFirstPersonPlayer_BP (Game|Player|GetPlayerPawn 0)))
  (Variables|Default|SetBossFirstPersonPlayer _asboss_first_person_player_bp)
  (Development|PrintString "Hello")
  (bind _returnvalue (Audio|SpawnSoundatLocation "/Game/DialogoSistem/Sounds/Phone/telephone-ringwav-14674.telephone-ringwav-14674" (Transformation|GetWorldLocation _cube) (Transformation|GetWorldRotation _cube) 1.0 1.0 0.0 0 0 false))
  (Variables|Default|SetRingPhoneSound _returnvalue))

(event EventInterfaceToggleFocus
  (params (Focus :type Boolean))
  (Rendering|SetRenderCustomDepth (Variables|Default|GetCube) Focus))

(event EventInterfaceInteract
  (CallFunction|InteractonServer))

(fn ConstructionScript
  (bind _returnvalue (Actor|GetActorOfClass "/Game/Players/UnmovilePlayers/BossRoomCommand_BP.BossRoomCommand_BP_C"))
  (Variables|Default|SetBossRoomChairPlayer _returnvalue))

(fn OnRepInteractToggle
  (bind _bossfirstpersonplayer (Variables|Default|GetBossFirstPersonPlayer))
  ;[0 0 0] Aqui es donde se debe poner la accion a realizar una vez se pulse el boton, si se pulsa es "True" si se vuelve a pulsar es "False".
  (if (Variables|Default|GetInteractToggle)
    _
    (else
      _))
  (Audio|Components|Audio|Stop (Variables|Default|GetRingPhoneSound))
  (Variables|Default|SetInPhone true)
  (Variables|Default|SetStopDialogue false)
  (if (Variables|/Game/Players/FistPersonPlayers/BossFirstPersonPlayer_BP.BossFirstPersonPlayer_BP_C|GetGanasteMusic _bossfirstpersonplayer)
    _
    (else
      (Audio|Components|Audio|FadeOut (Variables|/Game/Players/FistPersonPlayers/BossFirstPersonPlayer_BP.BossFirstPersonPlayer_BP_C|GetRoomMusic _bossfirstpersonplayer) 2.0 0.0 "SCurve" :!class /Script/Engine.AudioComponent)))
  (bind _returnvalue (UserInterface|CreateWidget "/Game/DialogoSistem/Widgets/HUD_Dialogue_WBP.HUD_Dialogue_WBP_C"))
  (bind _output_get (Variables|Default|SetHUD_DialogueRef _returnvalue))
  (bind _asbattle_gm (Utilities|Casting|CastToBattle_GM (Game|GetGameMode)))
  (Default|SetHUDDialogue _asbattle_gm _output_get)
  (UserInterface|Viewport|AddtoViewport _output_get 0))

(fn GameModeRef
  (return self))
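; Interactable first-person actor in the Boss Room that triggers the end of the game and returns to the main menu.
; Focus highlights the cube through custom depth, and interacting flips InteractToggle via InteractOnServer.
; Its OnRep, regardless of toggle value, fades out room music and the camera, then calls End.
; End hides the widget, then after delays shows the Teasendieron screen with a cheering sound and loads MainMenu3D.
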(event Custom|InteractOnServer
  (Variables|Default|SetInteractToggle (not (Variables|Default|GetInteractToggle))))

(event Custom|End
  (Development|SetHiddeninGame (Variables|Default|GetWidget) true false)
  (Utilities|FlowControl|Delay 4.0)
  (bind _returnvalue (UserInterface|CreateWidget "/Game/WINSCREEN/Widget/Teasendieron_WBP.Teasendieron_WBP_C"))
  (UserInterface|Viewport|AddtoViewport _returnvalue 0)
  (Audio|PlaySound2D "/Game/WINSCREEN/sounds/Niños_gritando_-_Kids_Yeah_Sound.Niños_gritando_-_Kids_Yeah_Sound" 1.0 1.0 0.0 0 0)
  (Utilities|FlowControl|Delay 5.0)
  (Game|OpenLevel(byName) "MainMenu3D"))

(event EventBeginPlay
  (bind _asboss_first_person_player_bp (Utilities|Casting|CastToBossFirstPersonPlayer_BP (Game|Player|GetPlayerPawn 0)))
  (Variables|Default|SetBossFirstPersonPlayer _asboss_first_person_player_bp))

(event EventInterfaceToggleFocus
  (params (Focus :type Boolean))
  (Rendering|SetRenderCustomDepth (Variables|Default|GetCube) Focus))

(event EventInterfaceInteract
  (CallFunction|InteractonServer))

(fn ConstructionScript
  (bind _returnvalue (Actor|GetActorOfClass "/Game/Players/UnmovilePlayers/BossRoomCommand_BP.BossRoomCommand_BP_C"))
  (Variables|Default|SetBossRoomChairPlayer _returnvalue))

(fn OnRepInteractToggle
  ;[0 0 0] Aqui es donde se debe poner la accion a realizar una vez se pulse el boton, si se pulsa es "True" si se vuelve a pulsar es "False".
  (if (Variables|Default|GetInteractToggle)
    _
    (else
      _))
  (Audio|Components|Audio|FadeOut (Variables|/Game/Players/FistPersonPlayers/BossFirstPersonPlayer_BP.BossFirstPersonPlayer_BP_C|GetRoomMusic (Variables|Default|GetBossFirstPersonPlayer)) 3.0 0.0 "Linear" :!class /Script/Engine.AudioComponent)
  (CameraFades|StartCameraFade :self (Game|GetPlayerCameraManager 0) :ToAlpha 1.0 :Duration 4.0 :bHoldWhenFinished true)
  (CallFunction|End))
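; ButtonTV3_ABP is an interactable button in the first-person boss room that switches the TV1 screen to the Nexo material.
; Interface events highlight the cube through custom depth on focus and call InteractOnServer, which flips InteractToggle.
; Its OnRep runs DelayMaterial on either value, showing static, then white, then the Nexo material with short delays.
; The construction script finds the screen and BossRoomCommand actors by class.
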(event Custom|InteractOnServer
  (Variables|Default|SetInteractToggle (not (Variables|Default|GetInteractToggle))))

(event Custom|DelayMaterial
  (Rendering|Material|SetMaterial (Variables|/Game/BossRoom/Interaction/InteractionActors/FPS/ScreenTV1_ABP.ScreenTV1_ABP_C|GetCube (Variables|Default|GetTV1)) 0 "/Game/BossRoom/SecurityCameras/Materials/StaticTV_M.StaticTV_M")
  (Utilities|FlowControl|Delay 0.5)
  (Rendering|Material|SetMaterial (Variables|/Game/BossRoom/Interaction/InteractionActors/FPS/ScreenTV1_ABP.ScreenTV1_ABP_C|GetCube (Variables|Default|GetTV1)) 0 "/Game/BossRoom/SecurityCameras/Materials/White_MI.White_MI")
  (Utilities|FlowControl|Delay 0.2)
  (Rendering|Material|SetMaterial (Variables|/Game/BossRoom/Interaction/InteractionActors/FPS/ScreenTV1_ABP.ScreenTV1_ABP_C|GetCube (Variables|Default|GetTV1)) 0 "/Game/BossRoom/SecurityCameras/Materials/NexoTV_M.NexoTV_M"))

(event EventInterfaceToggleFocus
  (params (Focus :type Boolean))
  (Rendering|SetRenderCustomDepth (Variables|Default|GetCube) Focus))

(event EventInterfaceInteract
  (CallFunction|InteractonServer))

(event EventBeginPlay
  (bind _asboss_first_person_player_bp (Utilities|Casting|CastToBossFirstPersonPlayer_BP (Game|Player|GetPlayerPawn 0)))
  (Variables|Default|SetBossFirstPersonPlayer _asboss_first_person_player_bp))

(fn ConstructionScript
  (bind _returnvalue (Actor|GetActorOfClass "/Game/Players/UnmovilePlayers/BossRoomCommand_BP.BossRoomCommand_BP_C"))
  (Variables|Default|SetBossRoomCommand _returnvalue)
  (bind _returnvalue_2 (Actor|GetActorOfClass "/Game/BossRoom/Interaction/InteractionActors/FPS/ScreenTV1_ABP.ScreenTV1_ABP_C"))
  (Variables|Default|SetTV1 _returnvalue_2)
  (Variables|Default|SetScreenLocation (Transformation|GetWorldLocation (Variables|Default|GetCube))))

(fn OnRepInteractToggle
  ;[0 0 0] Aqui es donde se debe poner la accion a realizar una vez se pulse el boton, si se pulsa es "True" si se vuelve a pulsar es "False".
  (if (Variables|Default|GetInteractToggle)
    (CallFunction|DelayMaterial)
    (else
      (CallFunction|DelayMaterial))))
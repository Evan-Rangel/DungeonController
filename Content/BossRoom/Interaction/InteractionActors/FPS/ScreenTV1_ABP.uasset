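; Interactable TV screen actor in the boss room that highlights on focus and drives the command actor's screen view.
; Interacting calls InteractOnServer to flip InteractToggle, whose OnRep calls GoToScreen and ReturnFromScreen on BossRoomCommand around a DelayMaterial call.
; DelayMaterial cycles timed static, white and battle materials, without delaying the return call.
; Toggling on also starts Battle_GM's Gestion phase first, stopping if that game mode cast fails.
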(event Custom|InteractOnServer
  (Variables|Default|SetInteractToggle (not (Variables|Default|GetInteractToggle))))

(event Custom|DelayMaterial
  (Utilities|FlowControl|Delay 1.0)
  (Rendering|Material|SetMaterial (Variables|Default|GetCube) 0 "/Game/BossRoom/SecurityCameras/Materials/StaticTV_M.StaticTV_M")
  (Utilities|FlowControl|Delay 2.0)
  (Rendering|Material|SetMaterial (Variables|Default|GetCube) 0 "/Game/BossRoom/SecurityCameras/Materials/White_MI.White_MI")
  (Utilities|FlowControl|Delay 2.0)
  (Rendering|Material|SetMaterial (Variables|Default|GetCube) 0 "/Game/BossRoom/SecurityCameras/Materials/BattleTV_M.BattleTV_M"))

(event EventInterfaceToggleFocus
  (params (Focus :type Boolean))
  (Rendering|SetRenderCustomDepth (Variables|Default|GetCube) Focus))

(event EventInterfaceInteract
  (CallFunction|InteractonServer))

(event EventBeginPlay
  (bind _asboss_first_person_player_bp (Utilities|Casting|CastToBossFirstPersonPlayer_BP (Game|Player|GetPlayerPawn 0)))
  (Variables|Default|SetBossFirstPersonPlayer _asboss_first_person_player_bp))

(fn ConstructionScript
  (bind _returnvalue (Actor|GetActorOfClass "/Game/Players/UnmovilePlayers/BossRoomCommand_BP.BossRoomCommand_BP_C"))
  (Variables|Default|SetBossRoomCommand _returnvalue)
  (Variables|Default|SetScreenLocation (Transformation|GetWorldLocation (Variables|Default|GetCube))))

(fn OnRepInteractToggle
  ;[0 0 0] Aqui es donde se debe poner la accion a realizar una vez se pulse el boton, si se pulsa es "True" si se vuelve a pulsar es "False".
  (if (Variables|Default|GetInteractToggle)
    (bind _asbattle_gm (Utilities|Casting|CastToBattle_GM (Game|GetGameMode)))
    (Default|StartGestionPhase _asbattle_gm)
    (Default|GotoScreen (Variables|Default|GetBossRoomCommand))
    (CallFunction|DelayMaterial)
    (Default|ReturnfromScreen (Variables|Default|GetBossRoomCommand))
    (else
      (Default|GotoScreen (Variables|Default|GetBossRoomCommand))
      (CallFunction|DelayMaterial)
      (Default|ReturnfromScreen (Variables|Default|GetBossRoomCommand)))))
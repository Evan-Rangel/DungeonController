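; Interactable command chair in the boss room that switches the player between the first-person pawn and the chair pawn.
; Focus toggles custom depth on its cube, and interaction calls InteractOnServer to flip InteractToggle.
; The toggle's RepNotify possesses either pawn with player controller 0, repositions the first-person pawn and updates camera limits, interaction trace and chair length distance.
; The chair pawn is found by class in the construction script.
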(event Custom|InteractOnServer
  (Variables|Default|SetInteractToggle (not (Variables|Default|GetInteractToggle))))

(event EventBeginPlay
  (bind _asboss_first_person_player_bp (Utilities|Casting|CastToBossFirstPersonPlayer_BP (Game|Player|GetPlayerPawn 0)))
  (Variables|Default|SetBossFirstPersonPlayer _asboss_first_person_player_bp))

(event EventInterfaceToggleFocus
  (params (Focus :type Boolean))
  (Rendering|SetRenderCustomDepth (Variables|Default|GetCube) Focus))

(event EventInterfaceInteract
  (CallFunction|InteractonServer))

(fn ConstructionScript
  (bind _returnvalue (Actor|GetActorOfClass "/Game/Players/UnmovilePlayers/BossRoomCommand_BP.BossRoomCommand_BP_C"))
  (Variables|Default|SetBossRoomChairPlayer _returnvalue))

(fn OnRepInteractToggle
  (bind _bossfirstpersonplayer (Variables|Default|GetBossFirstPersonPlayer))
  (bind _bossroomchairplayer (Variables|Default|GetBossRoomChairPlayer))
  ;[0 0 0] Aqui es donde se debe poner la accion a realizar una vez se pulse el boton, si se pulsa es "True" si se vuelve a pulsar es "False".
  (if (Variables|Default|GetInteractToggle)
    (Pawn|Possess (Game|GetPlayerController 0) _bossroomchairplayer)
    (Default|CameraLimitations _bossroomchairplayer)
    (Transformation|SetActorLocation (Variables|Default|GetBossFirstPersonPlayer) "100.000000,2500.000000,100.000000" false false)
    (Default|SetupInteractionTrace (Variables|Default|GetBossRoomChairPlayer))
    (Default|LenghtDistanceMax (Variables|Default|GetBossRoomChairPlayer))
    (else
      (Pawn|Possess (Game|GetPlayerController 0) _bossfirstpersonplayer)
      (Default|DefaultCameraLimitations _bossfirstpersonplayer)
      (Transformation|SetActorLocation (Variables|Default|GetBossFirstPersonPlayer) "760.000000,2500.000000,100.000000" false false)
      (Transformation|SetActorRotation (Variables|Default|GetBossFirstPersonPlayer))
      (Default|SetupInteractionTrace (Variables|Default|GetBossFirstPersonPlayer))
      (Default|LenghtDistanceMin (Variables|Default|GetBossRoomChairPlayer)))))
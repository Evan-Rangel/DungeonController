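; BattlePlayer_BP is a player-controlled actor for battle that turns key and mouse input into game-management commands.
; It forwards input to GestionGameC to toggle the building panel, change minion selection with the mouse wheel and request a new hero.
; Q makes the player controller possess the BossRoomCommand_BP actor, which the construction script finds by class.
; A comment flags some bindings as Evan's temporary ones.
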(event Input|MouseEvents|MouseWheelAxis
  (params (AxisValue :type Float%20%28single-precision%29))
  ;[0 0 0] Estos son temporales de Evan
  (Default|AddMinionSelection (Variables|Default|GetGestion%20Game%20C) AxisValue))

(event Input|KeyboardEvents|Q
  (params (Key :type Key%20Structure :default "None"))
  (:Pressed
    (Pawn|Possess (Game|GetPlayerController 0) (Variables|Default|GetBossRoomCommand))))

(event Input|MouseEvents|LeftMouseButton
  (params (Key :type Key%20Structure :default "None"))
  ;[0 0 0] Estos son temporales de Evan
  (:Pressed
    (Default|ActivateBuidingPanel (Variables|Default|GetGestion%20Game%20C) false)))

(event Input|MouseEvents|RightMouseButton
  (params (Key :type Key%20Structure :default "None"))
  ;[0 0 0] Estos son temporales de Evan
  (:Pressed
    (Default|ActivateBuidingPanel (Variables|Default|GetGestion%20Game%20C) true)))

(event Input|KeyboardEvents|C
  (params (Key :type Key%20Structure :default "None"))
  ;[0 0 0] Estos son temporales de Evan
  (:Pressed
    (Default|RequestNewHeroG (Variables|Default|GetGestion%20Game%20C))))

(event Input|KeyboardEvents|SpaceBar
  (params (Key :type Key%20Structure :default "None"))
  (:Pressed
    ;[0 0 0] Estos son temporales de Evan
    (Default|ActivateBuidingPanel (Variables|Default|GetGestion%20Game%20C) false)))

(event Input|KeyboardEvents|Z
  (params (Key :type Key%20Structure :default "None"))
  ;[0 0 0] Estos son temporales de Evan
  (:Pressed
    (Default|ActivateBuidingPanel (Variables|Default|GetGestion%20Game%20C) true)))

(event Input|KeyboardEvents|X
  (params (Key :type Key%20Structure :default "None"))
  (:Pressed
    ;[0 0 0] Estos son temporales de Evan
    (Default|ActivateBuidingPanel (Variables|Default|GetGestion%20Game%20C) false)))

(fn ConstructionScript
  (bind _returnvalue (Actor|GetActorOfClass "/Game/Players/UnmovilePlayers/BossRoomCommand_BP.BossRoomCommand_BP_C"))
  (Variables|Default|SetBossRoomCommand _returnvalue))
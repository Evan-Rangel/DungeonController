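; Menu3D_ABP is a 3D main menu actor that hosts a Menu3D_WBP widget and moves the view to linked menus.
; On BeginPlay it binds to the widget's TransitionToLinkedMenu dispatcher, and a menu index selects the target from LinkedMenus.
; A transition disables its own collision, enables the target's, and eases the player's view target to that actor with a camera blend.
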(event Custom|TransitionTo
  (params (Menu3D :type Menu%203D%20ABP%20Object%20Reference))
  (Collision|SetActorEnableCollision false)
  (Collision|SetActorEnableCollision Menu3D true)
  (Game|Player|SetViewTargetwithBlend (Game|GetPlayerController 0) Menu3D 2.0 "VTBlend_EaseInOut" 2.0 false))

(event Custom|OnTransitionBetweenMenus
  (params (MenuIndex :type Integer))
  (if (Utilities|Array|IsValidIndex (Variables|Default|GetLinkedMenus) MenuIndex)
    (CallFunction|Transitionto (Utilities|Array|Get(acopy) (Variables|Default|GetLinkedMenus) MenuIndex))))

(event EventBeginPlay
  (bind _asmenu_3d_wbp (Utilities|Casting|CastToMenu3D_WBP (UserInterface|GetUserWidgetObject (Variables|Default|GetWidget))))
  (EventDispatchers|AssignTransitiontoLinkedMenu _asmenu_3d_wbp (EventDispatchers|CreateEvent :!event Custom|OnTransitionBetweenMenus))
  (Actor|GetActorOfClass 0))

(fn ConstructionScript)
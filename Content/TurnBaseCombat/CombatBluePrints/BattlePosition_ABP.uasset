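; Battle position marker actor that spawns a combat unit at its transform for turn-based battles.
; The construction script colors its arrow blue or red based on IsHeroPlacement to distinguish heroes from villains in the editor.
; SpawnUnit spawns a valid UnitClass, passes health, mana, level and XP from its input to the unit's EventSetStats, and returns the unit.
; BeginPlay is empty, so spawning relies on an external call.
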(event EventBeginPlay
  ;[0 0 0] Llama a la funcion de "SpawnUnit" para nadamas comenzar se posicionen los personajes.
)

(fn ConstructionScript
  ;[0 0 0] "Construction Script" toma la Flecha que simboliza a las unidades y le da un color dependiendo si es un Heroe o un Villano.
  (Components|Arrow|SetArrowColor(LinearColor) (Variables|Default|GetArrow) (Math|Color|SelectColor "(R=0.000000,G=0.000000,B=1.000000,A=1.000000)" "(R=1.000000,G=0.000000,B=0.000000,A=1.000000)" (Variables|Default|GetisHeroPlacement))))

(fn SpawnUnit
  (params (_Min :type Minion%20Object%20Reference))
  ;[0 0 0] "SpawnUnit" sera llamada al iniciar la batalla, para que asi pueda spawnear las unidades en sus respectivas posiciones, Heroes a la izquierda, Villanos a la derecha.
  (bind _unitclass (Variables|Default|GetUnitClass)
    (:then
      (bind _returnvalue (Game|SpawnActorfromClass _unitclass (Transformation|GetActorTransform) "AdjustIfPossibleButAlwaysSpawn" "MultiplyWithRoot" 0 0))
      (Default|EventSetStats _returnvalue (Math|Conversions|ToFloat(Integer) (Variables|/Game/Grid/Minion.Minion_C|GetMaxHealth _Min)) (Math|Conversions|ToFloat(Integer) (Variables|/Game/Grid/Minion.Minion_C|GetHealth _Min)) (Math|Conversions|ToFloat(Integer) (Variables|/Game/Grid/Minion.Minion_C|GetMaxMana _Min)) (Math|Conversions|ToFloat(Integer) (Variables|/Game/Grid/Minion.Minion_C|GetMana _Min)) (Variables|/Game/Grid/Minion.Minion_C|GetLevel _Min) (Variables|/Game/Grid/Minion.Minion_C|GetXP _Min))
      (return _returnvalue))
    (:else)))
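; Projectile actor for turn-based combat that delivers its instigator's attack damage when it hits.
; On spawn, its sphere ignores the instigator while moving so the shooter does not block its path.
; On hit, it gets damage from the instigator's BattleAC and applies it to that component's UnitTarget, regardless of what was struck.
; It spawns the impact effect at the target's location, then destroys itself after a short delay.
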(event EventBeginPlay
  ;[0 0 0] Se inicializa con el actor con un "IgnoreActorwhenMoving" para evitar que su trayectoria se vea afectada.
  (Collision|IgnoreActorwhenMoving (Variables|Default|GetSphere) (Game|GetInstigator) true))

(event Collision|EventHit
  (params (MyComp :type Primitive%20Component%20Object%20Reference) (Other :type Actor%20Object%20Reference) (OtherComp :type Primitive%20Component%20Object%20Reference) (bSelfMoved :type Boolean) (HitLocation :type Vector :default "0, 0, 0") (HitNormal :type Vector :default "0, 0, 0") (NormalImpulse :type Vector :default "0, 0, 0") (Hit :type Hit%20Result%20Structure%20%28by%20ref%29))
  ;[0 0 0] "Event Hit" empieza con un "SpawnEmitteratLocation" el cual se le da la variable "ImpactEffect" que es quien guarda el efecto de disparo, despues se llama a la funcion "CalculateDamage" que esta en "Battle_AC", luego se llama a la funcion de "ApplyDamage", se llenan los valores de la misma forma como ocurrio en "DealDamage_NBP", se le da un delay y se destruye el proyectil.
  (bind _asunit_base_cbp (Utilities|Casting|CastToUnitBase_CBP (Game|GetInstigator)))
  (bind _basedamage (Default|CalculateDamage (Variables|/Game/TurnBaseCombat/CombatBluePrints/UnitBase_CBP.UnitBase_CBP_C|GetBattle_AC _asunit_base_cbp)))
  (Game|Damage|ApplyDamage (Variables|/Game/TurnBaseCombat/CombatBluePrints/Batlle_AC.Batlle_AC_C|GetUnitTarget (Variables|/Game/TurnBaseCombat/CombatBluePrints/UnitBase_CBP.UnitBase_CBP_C|GetBattle_AC _asunit_base_cbp)) _basedamage 0 _asunit_base_cbp (Variables|Default|GetDamage%20Type%20Class))
  (Effects|SpawnEmitteratLocation (Variables|Default|GetImpactEffect) (Transformation|GetActorLocation (Variables|/Game/TurnBaseCombat/CombatBluePrints/Batlle_AC.Batlle_AC_C|GetUnitTarget (Variables|/Game/TurnBaseCombat/CombatBluePrints/UnitBase_CBP.UnitBase_CBP_C|GetBattle_AC _asunit_base_cbp))))
  (Utilities|FlowControl|Delay 1.0)
  (Actor|DestroyActor))

(fn ConstructionScript)
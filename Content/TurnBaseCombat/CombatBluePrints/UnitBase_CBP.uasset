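; Base unit Blueprint for turn-based combat, holding HP, MP, level and XP.
; AnyDamage applies BattleAC resistance, clamps HP, spawns damage-number widgets and drives low-HP stun or death montages, with death removing the unit through Battle_GM.
; CheckForStun replays the stun montage at low HP, and CalculateSpendMP deducts spell costs.
; ChooseLoot makes a weighted random pick from the LootTable map.
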(event Custom|CheckForStun
  ;[0 0 0] Para Evitar que ataque un enemigo Stunneado que ya habia pedido un turno se hace un evento que revisa si esta Stuneado o no y se llama en "Battle_AC" en la funcion "EndUnitTurn".
  (if (Math|Float|InRange(Float) (Variables|CharacterInfo|GetCurrent_HP) 0.0 (* (Variables|CharacterInfo|GetMax_HP) 0.1) false)
    (Animation|Montage|PlayMontage (Variables|Character|GetMesh) (Variables|CharacterAnimations|GetStunAnimation))))

(event Custom|Event%20OnSpawn
  (params (Max_HP :type Float%20%28double-precision%29) (Current_HP :type Float%20%28double-precision%29) (Max_MP :type Float%20%28double-precision%29) (Current_MP :type Float%20%28double-precision%29) (Lvl :type Integer) (TXP :type Integer))
  (Variables|CharacterInfo|SetMax_HP Max_HP)
  (Variables|CharacterInfo|SetCurrent_HP Current_HP)
  (Variables|CharacterInfo|SetMax_MP Max_MP)
  (Variables|CharacterInfo|SetCurrent_MP Current_MP)
  (Variables|CharacterInfo|SetTLvl Lvl)
  (Variables|CharacterInfo|SetTXP TXP))

(event Custom|Event%20SetStats
  (params (Max_HP :type Float%20%28double-precision%29) (Current_HP :type Float%20%28double-precision%29) (Max_MP :type Float%20%28double-precision%29) (Current_MP :type Float%20%28double-precision%29) (Lvl :type Integer) (TXP :type Integer))
  ;[0 0 0] Se multiplican los valores de HP y MP en el "BeginPlay" pa iniciar con sus valores correspondientes.
  (Variables|CharacterInfo|SetMax_HP Max_HP)
  (Variables|CharacterInfo|SetCurrent_HP Current_HP)
  (Variables|CharacterInfo|SetMax_MP Max_MP)
  (Variables|CharacterInfo|SetCurrent_MP Current_MP)
  (Variables|CharacterInfo|SetTLvl Lvl)
  (Variables|CharacterInfo|SetTXP TXP)
  (Default|GetLevel (Variables|Default|GetBattle_AC)))

(event EventBeginPlay
  ;[0 0 0] Se multiplican los valores de HP y MP en el "BeginPlay" pa iniciar con sus valores correspondientes.
)

(event EventTick
  (params (DeltaSeconds :type Float%20%28single-precision%29)))

(event Game|Damage|EventAnyDamage
  (params (Damage :type Float%20%28single-precision%29) (DamageType :type Damage%20Type%20Object%20Reference) (InstigatedBy :type Controller%20Object%20Reference) (DamageCauser :type Actor%20Object%20Reference))
  ;[0 0 0] "EventAnyDamage" es un evento predefinido de UnrealEngine, aqui es utilizado para que cuando el evento es llamado se obtenga la variable "HitReactAnimation" la cual guarda una animacion, comprobamos si es valido y se reproduce la animacion en la unidad correspondiente.
  (Utilities|FlowControl|Sequence
    (:then_0
      (if (< Damage 0.0)
        (bind _hitreactanimation (Variables|CharacterAnimations|GetHitReactAnimation)
          (:then
            (Animation|Montage|PlayMontage (Variables|Character|GetMesh) _hitreactanimation))
          (:else))))
    (:then_1
      (bind _finaldamage (Default|CalculateDamageResistance (Variables|Default|GetBattle_AC) Damage))
      (Variables|CharacterInfo|SetCurrent_HP (Math|Float|Clamp(Float) (- (Variables|CharacterInfo|GetCurrent_HP) _finaldamage) 0.0 (Variables|CharacterInfo|GetMax_HP)))
      (Utilities|FlowControl|Sequence
        (:then_0
          (bind _returnvalue (UserInterface|CreateWidget "/Game/TurnBaseCombat/CombatUI/DamageNumbers_WBP.DamageNumbers_WBP_C" 0 _finaldamage self))
          (UserInterface|Viewport|AddtoViewport _returnvalue 0))
        (:then_1
          (if (Math|Float|InRange(Float) (Variables|CharacterInfo|GetCurrent_HP) 0.0 (* (Variables|CharacterInfo|GetMax_HP) 0.1) false)
            (Animation|Montage|PlayMontage (Variables|Character|GetMesh) (Variables|CharacterAnimations|GetStunAnimation))
            (elif (<= (Variables|CharacterInfo|GetCurrent_HP) 0.0)
              (Animation|Montage|PlayMontage (Variables|Character|GetMesh) (Variables|CharacterAnimations|GetDieAnimation)
                (:then
                  (Pawn|UnPossess (AI|GetAIController self))
                  (bind _asbattle_gm (Utilities|Casting|CastToBattle_GM (Game|GetGameMode)))
                  (Default|RemoveUnitfromBattle _asbattle_gm self)))
              (elif (Animation|Montage|MontageIsPlaying (Components|SkeletalMesh|GetAnimInstance (Variables|Character|GetMesh)) (Variables|CharacterAnimations|GetStunAnimation))
                (Animation|Montage|PlayMontage (Variables|Character|GetMesh) (Variables|CharacterAnimations|GetStunAnimation) 1.0 0.0 "ExitStun")))))))))

(fn ConstructionScript)

(fn CalculateSpendMP
  (params (MPCost :type Float%20%28double-precision%29))
  ;[0 0 0] "CalculateSpendMP" es una funcion para que los ataques magicos gasten su respectivo MP al ser usados, su costo puede sr visto en el respectivo ataque magico y esta funcion es llamada en la UI de "HeroesUISlot_WBP".
  (Variables|CharacterInfo|SetCurrent_MP (Math|Float|Clamp(Float) (- (Variables|CharacterInfo|GetCurrent_MP) MPCost) 0.0 (Variables|CharacterInfo|GetMax_MP)))
  (Default|CallMPSpent))

(fn ChooseLoot
  (bind _loottable (Variables|CharacterInfo|GetLootTable))
  (bind _loottable_2 (Variables|CharacterInfo|GetLootTable))
  ;[0 0 0] Por cada objeto se le aplicaran llaves las cuales con un numero random se iran seleccionando, depende de cuantos llaves vale cada objeto para asi determinar su posibilidad de salir.
  (Utilities|FlowControl|Sequence
    (:then_0
      (bind _keys (Utilities|Map|Keys _loottable))
      (for _array_element _keys
        (LocalVariables|SetSum_Loc (+ (LocalVariables|GetSum_Loc) (.Value (Utilities|Map|Find _loottable _array_element))))))
    (:then_1
      (LocalVariables|SetRandomValue_Loc (Math|Random|RandomFloatinRange 0.0 (LocalVariables|GetSum_Loc)))
      (bind _keys_2 (Utilities|Map|Keys _loottable_2))
      (for _array_element_2 _keys_2
        (if (< (LocalVariables|GetRandomValue_Loc) (.Value (Utilities|Map|Find _loottable_2 _array_element_2)))
          (return _array_element_2)
          (else
            (LocalVariables|SetRandomValue_Loc (- (LocalVariables|GetRandomValue_Loc) (.Value (Utilities|Map|Find _loottable_2 _array_element_2))))))))))
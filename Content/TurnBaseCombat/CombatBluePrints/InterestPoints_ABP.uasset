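; InterestPoints_ABP is a clickable interest point sphere, apparently marking a country, that reports selection to the player's UserMenu_BP pawn.
; BeginPlay caches that pawn and the sphere's world location and rotation.
; Cursor hover raises and restores the material's glow through scalar parameters.
; A click passes the point to ClickOnInterestPointMessage and runs a timeline that drives material opacity, then deactivates the sphere component.
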(event OnBeginCursorOver(Sphere)
  (params (TouchedComponent :type Primitive%20Component%20Object%20Reference))
  ;[0 0 0] Al tener el cursor en el objeto brillara mas, y al dejar de tenerlo vuelve a su brillo original
  (Rendering|Material|SetScalarParameterValueonMaterials (Variables|Default|GetSphere) "Glow Intensity" 5e+01))

(event OnEndCursorOver(Sphere)
  (params (TouchedComponent :type Primitive%20Component%20Object%20Reference))
  ;[0 0 0] Al tener el cursor en el objeto brillara mas, y al dejar de tenerlo vuelve a su brillo original
  (Rendering|Material|SetScalarParameterValueonMaterials (Variables|Default|GetSphere) "Glow Intensity" 1e+01))

(event OnClicked(Sphere)
  (params (TouchedComponent :type Primitive%20Component%20Object%20Reference) (ButtonPressed :type Key%20Structure :default "None"))
  ;[0 0 0] Al hacer click se hace un llamado a "ClickOnCountry" para que haga el movimiento de camara.
  (Class|ClickInterestPointIF|ClickonInterestPoint(Message) (Variables|UserPlayer|GetUserMenu) self)
  (bind _fade (Timeline|FadeCountryPoint Play)
    (:Update
      (Rendering|Material|SetScalarParameterValueonMaterials (Variables|Default|GetSphere) "Opacity" _fade))
    (:Finished
      (Components|Activation|SetActive (Variables|Default|GetSphere) false false))))

(event EventBeginPlay
  ;[0 0 0] Se inicia un caste al Usuario
  (bind _asuser_menu_bp (Utilities|Casting|CastToUserMenu_BP (Game|Player|GetPlayerPawn 0)))
  (Variables|UserPlayer|SetUserMenu _asuser_menu_bp)
  (Variables|PointsInfo|SetCountryPointsLocation (Transformation|GetWorldLocation (Variables|Default|GetSphere)))
  (Variables|PointsInfo|SetCountryPointsRotation (Transformation|GetWorldRotation (Variables|Default|GetSphere))))

(fn ConstructionScript)
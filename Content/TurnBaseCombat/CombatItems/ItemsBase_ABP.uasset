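; Base actor for turn-based combat items, consumed from the player's inventory when spawned.
; On BeginPlay it finds the GestionGameController and, if its own class is a key in the ItemsInventory map, lowers that count by one.
; The actor destroys itself when either its Niagara or its ParticleSystem component finishes playing, so its lifetime follows the visual effect.
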(event OnSystemFinished(Niagara)
  (params (PSystem :type Niagara%20Component%20Object%20Reference))
  (Actor|DestroyActor))

(event OnSystemFinished(ParticleSystem)
  (params (PSystem :type Particle%20System%20Component%20Object%20Reference))
  (Actor|DestroyActor))

(event EventBeginPlay
  (bind _self self)
  (bind _returnvalue (Utilities|GetClass _self))
  (bind _returnvalue_2 (Actor|GetActorOfClass "/Game/Grid/GestionGameController.GestionGameController_C"))
  (if (.ReturnValue (Utilities|Map|Find (Variables|/Game/Grid/GestionGameController.GestionGameController_C|GetItemsInventory _returnvalue_2) _returnvalue))
    (Utilities|Map|Add (Variables|/Game/Grid/GestionGameController.GestionGameController_C|GetItemsInventory _returnvalue_2) _returnvalue (- (.Value (Utilities|Map|Find (Variables|/Game/Grid/GestionGameController.GestionGameController_C|GetItemsInventory _returnvalue_2) _returnvalue)) 1))))

(event Collision|EventActorBeginOverlap
  (params (OtherActor :type Actor%20Object%20Reference)))

(event EventTick
  (params (DeltaSeconds :type Float%20%28single-precision%29)))

(fn ConstructionScript)
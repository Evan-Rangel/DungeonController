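; Protective Scroll is a turn-based combat support item actor that temporarily raises the DEF stat modifier of its recipient.
; On BeginPlay it adds a point of DEF to the recipient's BattleAC stats modifier and starts a one-shot 20-second timer, evidently for ItemDropOff.
; ItemDropOff reverses the bonus and destroys the actor, so the buff lasts by real time rather than turns.
; Niagara and particle components destroy themselves when their effects finish.
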(event OnSystemFinished(Niagara)
  (params (PSystem :type Niagara%20Component%20Object%20Reference))
  (Components|DestroyComponent PSystem))

(event OnSystemFinished(ParticleSystem)
  (params (PSystem :type Particle%20System%20Component%20Object%20Reference))
  (Components|DestroyComponent PSystem))

(event Custom|ItemDropOff
  (bind _recipient (Variables|Default|GetRecipient))
  (bind _battle_ac (Variables|/Game/TurnBaseCombat/CombatBluePrints/UnitBase_CBP.UnitBase_CBP_C|GetBattle_AC _recipient))
  (bind _unitstatsmodifier (Variables|/Game/TurnBaseCombat/CombatBluePrints/Batlle_AC.Batlle_AC_C|GetUnitStatsModifier _battle_ac))
  (bind _def (Utilities|Struct|BreakStatsModifierTable_S _unitstatsmodifier))
  ;[0 0 0] Este evento revierte el efecto aplicado.
  (Development|PrintString "se acabooooooo")
  (Utilities|Struct|SetmembersinStatsModifierTable_S _unitstatsmodifier (+ _def -1.0))
  (Development|PrintString (Utilities|String|ToString(Float) _def))
  (Actor|DestroyActor))

(event EventBeginPlay
  (bind _recipient (Variables|Default|GetRecipient))
  (bind _battle_ac (Variables|/Game/TurnBaseCombat/CombatBluePrints/UnitBase_CBP.UnitBase_CBP_C|GetBattle_AC _recipient))
  (bind _unitstatsmodifier (Variables|/Game/TurnBaseCombat/CombatBluePrints/Batlle_AC.Batlle_AC_C|GetUnitStatsModifier _battle_ac))
  (bind _def (Utilities|Struct|BreakStatsModifierTable_S _unitstatsmodifier))
  ;[0 0 0] Al usarse el objeto se aplica la modificacion de estadisticas de DEF, se pone un timer y se mantendra en escena el tiempo del timer, luego se llama al evento que revierte el effecto.
  (|CallParentFunction)
  (Utilities|Struct|SetmembersinStatsModifierTable_S _unitstatsmodifier (+ _def 1.0))
  (Development|PrintString (Utilities|String|ToString(Float) _def))
  (Utilities|Time|SetTimerbyEvent (EventDispatchers|CreateEvent :!event Custom|ItemDropOff) 2e+01))

(event Collision|EventActorBeginOverlap
  (params (OtherActor :type Actor%20Object%20Reference))
  (|CallParentFunction OtherActor) ; This node is disabled and will not be called.\nDrag off pins to build functionality.
)

(event EventTick
  (params (DeltaSeconds :type Float%20%28single-precision%29))
  (|CallParentFunction DeltaSeconds) ; This node is disabled and will not be called.\nDrag off pins to build functionality.
)

(fn ConstructionScript
  (|CallParentFunction))
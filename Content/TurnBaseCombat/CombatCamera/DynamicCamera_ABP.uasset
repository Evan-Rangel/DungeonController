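; Dynamic camera actor for turn-based combat that orbits, follows an actor or glides to a point.
; SetDynamicCameraLocation snaps and attaches it to a valid actor, otherwise detaches and sets a target location and look-at rotation.
; While unattached, Tick interpolates actor location and camera rotation toward those targets; SetLookatActor detaches and aims at an actor.
; SetOrbit toggles RotatingMovement spin and spring-arm yaw inheritance, resetting rotation when off.
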(event EventSetLookatActor
  (params (TargetActor :type Actor%20Object%20Reference))
  ;[1 1 1] Este target rotation va a ser usado para la animacion de la camara mirando, asi se podra setear a donde queremos que este mirando.
  (Variables|Default|SetTargetRotation (Math|Rotator|FindLookatRotation (Camera|GetCameraLocation (Game|GetPlayerCameraManager 0)) (Transformation|GetActorLocation TargetActor)))
  (Transformation|DetachFromActor "KeepWorld" "KeepWorld" "KeepWorld"))

(event EventSetOrbit
  (params (IsOrbiting :type Boolean))
  ;[1 1 1] Llamaos al evento para determinar la velocidad con la que la camara va a rotar. Ademas setear que ocurrira cuando no queremos que rote.
  (Variables|/Script/Engine.RotatingMovementComponent|SetRotationRate (Variables|Default|GetRotatingMovement) (Math|Rotator|SelectRotator "0.000000,10.000000,0.000000" "0, 0, 0" IsOrbiting))
  (bind _output_get (Variables|/Script/Engine.SpringArmComponent|SetbInheritYaw (Variables|Default|GetSpringArm) IsOrbiting))
  (if (not _output_get)
    (Transformation|SetActorRotation "0, 0, 0")))

(event EventSetDynamicCameraLocation
  (params (Actor :type Actor%20Object%20Reference) (Vector :type Vector :default "0, 0, 0"))
  ;[1 1 1] Si el evento es verdadero entonces el objeto de la camara sera attacheado a la unidad osea a otro actor.
  (Utilities|IsValid Actor
    (:Is%20Valid
      (Transformation|AttachActorToActor Actor "None" "SnapToTarget" "KeepWorld" "KeepWorld" true)
      (Transformation|SetRelativeRotation (Variables|Default|GetCamera) "0, 0, 0" false false)
      (Variables|Default|SetTargetLocation (Transformation|GetActorLocation Actor)))
    (:Is%20Not%20Valid
      (bind _output_get (Variables|Default|SetTargetLocation Vector))
      (Transformation|DetachFromActor "KeepWorld" "KeepWorld" "KeepWorld")
      (Variables|Default|SetTargetRotation (Math|Rotator|FindLookatRotation (Transformation|GetWorldLocation (Variables|Default|GetCamera)) _output_get)))))

(event EventTick
  (params (DeltaSeconds :type Float%20%28single-precision%29))
  ;[1 1 1] En el "EventTick" se estara comprobando si esta attacheado a un actor o no. Si es un no va a hacer un lerp a la locacion deseada.
  (Utilities|IsValid (Actor|GetAttachParentActor)
    (:Is%20Not%20Valid
      (Transformation|SetActorLocation (Math|Interpolation|VInterpTo (Transformation|GetActorLocation) (Variables|Default|GetTargetLocation) (Utilities|Time|GetWorldDeltaSeconds) 5.0) false false)
      (Transformation|SetWorldRotation (Variables|Default|GetCamera) (Math|Interpolation|RInterpTo (Transformation|GetWorldRotation (Variables|Default|GetCamera)) (Variables|Default|GetTargetRotation) (Utilities|Time|GetWorldDeltaSeconds) 5.0) false false))))

(fn ConstructionScript)
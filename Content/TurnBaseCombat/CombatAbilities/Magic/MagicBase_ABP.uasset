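; Base actor for magic abilities in turn-based combat, handling MP cost, sound and effect lifetime.
; On BeginPlay it casts its Instigator to UnitBase_CBP, looks up the cost for AbilityRank in MagicCostTable and passes it to that unit's CalculateSpendMP.
; It then plays the ability sound in 2D; if the cast fails, neither step runs.
; The actor destroys itself when either its particle system or Niagara effect finishes.
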(event OnSystemFinished(ParticleSystem)
  (params (PSystem :type Particle%20System%20Component%20Object%20Reference))
  ;[0 0 0] Cuando termina de ocurrir el efecto se destruye.
  (Actor|DestroyActor))

(event OnSystemFinished(Niagara)
  (params (PSystem :type Niagara%20Component%20Object%20Reference))
  ;[0 0 0] Cuando termina de ocurrir el efecto se destruye.
  (Actor|DestroyActor))

(event EventBeginPlay
  ;[0 0 0] Al iniciar el ataque se hara una busqueda entre la tabla de magias y el rango de la misma para determinar con cual de ellas se hara la funcion "CalculateSpendMP" para hacer la resta al MP de la unidad.
  (bind _asunit_base_cbp (Utilities|Casting|CastToUnitBase_CBP (Game|GetInstigator)))
  (Default|CalculateSpendMP _asunit_base_cbp (.Value (Utilities|Map|Find (Variables|MagicAbilitieStats|GetMagicCostTable) (Variables|MagicAbilitieInfo|GetAbilityRank))))
  (Audio|PlaySound2D (Variables|MagicSounds|GetMagicAbilitySound) 1.0 1.0 0.0 0 0))

(fn ConstructionScript)
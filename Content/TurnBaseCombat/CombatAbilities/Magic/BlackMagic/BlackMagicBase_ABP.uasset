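; BlackMagicBase_ABP is an actor, by its name the base for black magic abilities in turn-based combat, that deals magical damage when spawned.
; On BeginPlay it casts its instigator to UnitBase_CBP and has that unit's BattleAC calculate base damage from the spell's own class.
; It applies that damage to MagicTarget using its DamageTypeClass, with the instigator as damage causer.
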(event EventBeginPlay
  (bind _returnvalue (Game|GetInstigator))
  ;[0 0 0] Al iniciar el ataque magico se hara el calculo de daño con la funcion "CalculateMagicalBaseDamage" y esos valores seran llevados a "ApplyDamage".
  (|CallParentFunction)
  (bind _asunit_base_cbp (Utilities|Casting|CastToUnitBase_CBP _returnvalue))
  (bind _calculatedamage (Default|CalculateMagicalBaseDamage (Variables|/Game/TurnBaseCombat/CombatBluePrints/UnitBase_CBP.UnitBase_CBP_C|GetBattle_AC _asunit_base_cbp) (Utilities|GetClass self)))
  (Game|Damage|ApplyDamage (Variables|Default|GetMagicTarget) _calculatedamage 0 _returnvalue (Variables|Default|GetDamage%20Type%20Class)))

(fn ConstructionScript
  (|CallParentFunction))
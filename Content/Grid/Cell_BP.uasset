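; Grid cell actor for a battle map that can be empty, a wall or a building.
; A dynamic material on its plane, created in the construction script, lets ChangeColor switch empty cells between normal and selected colors.
; StartBuilding resets the level to one, then sets unit walkability from the cell type and a maximum level from the building type.
; BeginPlay applies the unselected color and caches the Battle_GM game mode.
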(event EventBeginPlay
  (CallFunction|ChangeColor false)
  (bind _asbattle_gm (Utilities|Casting|CastToBattle_GM (Game|GetGameMode)))
  (Variables|Default|SetGameManager _asbattle_gm))

(event Collision|EventActorBeginOverlap
  (params (OtherActor :type Actor%20Object%20Reference)))

(event EventTick
  (params (DeltaSeconds :type Float%20%28single-precision%29)))

(fn ConstructionScript
  ;[0 0 0] Crea el material dinamico para poder cambiar el color
  (bind _returnvalue (Rendering|Material|CreateDynamicMaterialInstance (Variables|Default|GetPlane1) 0 "/Engine/BasicShapes/BasicShapeMaterial.BasicShapeMaterial" "None" :!class /Script/Engine.PrimitiveComponent))
  (Variables|Colors|SetMat _returnvalue))

(fn ChangeColor
  (params (_IsSelect :type Boolean))
  ;[0 0 0] Cambia el color dependiendo del switch
  (switch Utilities|FlowControl|Switch|SwitchonCellType (Variables|CellConfig|GetCellType)
    (:NewEnumerator0
      (if _IsSelect
        (CallFunction|SetColor (Variables|Colors|GetSelectColor))
        (else
          (CallFunction|SetColor (Variables|Colors|GetNormalColor)))))))

(fn SetColor
  (params (NewParam :type Color%20Structure))
  ;[0 0 0] Funcion que recibe input para cambiar color el material
  (Rendering|Material|SetVectorParameterValue (Variables|Colors|GetMat) "Color" (Math|Conversions|ToLinearColor(Color) NewParam) :!class /Script/Engine.MaterialInstanceDynamic))

(fn StartBuilding
  (Variables|Resourses|SetLevel 1)
  (switch Utilities|FlowControl|Switch|SwitchonCellType (Variables|CellConfig|GetCellType)
    (:NewEnumerator1
      (Variables|CellConfig|SetUnitsCanWalk false))
    (:NewEnumerator3
      (Variables|CellConfig|SetUnitsCanWalk true)
      (switch Utilities|FlowControl|Switch|SwitchonBuildingType (Variables|CellConfig|GetBuildingType)
        (:NewEnumerator0
          (Variables|Resourses|SetMaxLevel 3))
        (:NewEnumerator1
          (Variables|Resourses|SetMaxLevel 3))
        (:NewEnumerator2
          (Variables|Resourses|SetMaxLevel 3))
        (:NewEnumerator3
          (Variables|Resourses|SetMaxLevel 5))
        (:NewEnumerator4
          (Variables|Resourses|SetMaxLevel 3))))))